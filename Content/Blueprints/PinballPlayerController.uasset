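; Player controller for a pinball game that routes player input to the table's flippers and plunger and shows the HUD.
; On BeginPlay it finds every flipper and sorts them into left and right arrays by type, grabs the first plunger found, and replaces all widgets with a new PinballHUD.
; Input actions flip and release each side's flippers, and start and stop charging the plunger.
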(event `GetPlayerHUD`
  (`WidgetLayoutLibrary.RemoveAllWidgets`)
  (bind _returnvalue (`|CreateWidget` "/Game/Blueprints/PinballHUD.PinballHUD_C"))
  (`UserWidget.AddToViewport` _returnvalue 0))

(event `DetectPlunger`
  (bind _outactors (`GameplayStatics.GetAllActorsOfClass` "/Game/Blueprints/BP_Plunger.BP_Plunger_C"))
  (set `self.Plunger` (`KismetArrayLibrary.Array_Get` _outactors)))

(event `self.ReceiveBeginPlay`
  (`self.DetectFlippers`)
  (`self.DetectPlunger`)
  (`self.GetPlayerHUD`))

(event `DetectFlippers`
  (bind _outactors (`GameplayStatics.GetAllActorsOfClass` "/Game/Blueprints/BP_Flipper.BP_Flipper_C"))
  (for _array_element _outactors
    (switch `/Game/Blueprints/FlipperType` (`/Game/Blueprints/BP_Flipper.FlipperType` _array_element)
      (:`NewEnumerator0`
        (`KismetArrayLibrary.Array_Add` (`self.LeftFlipper`) _array_element))
      (:`NewEnumerator1`
        (`KismetArrayLibrary.Array_Add` (`self.RightFlipper`) _array_element)))))

(event `InputAction|LeftFlipper`
  (params (Key :type "Key Structure" :default "AnyKey"))
  (bind _leftflipper (`self.LeftFlipper`))
  (:`Pressed`
    (for _array_element _leftflipper
      (`/Game/Blueprints/BP_Flipper.Flip` _array_element)))
  (:`Released`
    (for _array_element_2 _leftflipper
      (`/Game/Blueprints/BP_Flipper.Flop` _array_element_2))))

(event `InputAction|RightFlipper`
  (params (Key :type "Key Structure" :default "AnyKey"))
  (bind _rightflipper (`self.RightFlipper`))
  (:`Pressed`
    (for _array_element _rightflipper
      (`/Game/Blueprints/BP_Flipper.Flip` _array_element)))
  (:`Released`
    (for _array_element_2 _rightflipper
      (`/Game/Blueprints/BP_Flipper.Flop` _array_element_2))))

(event `InputAction|Plunger`
  (params (Key :type "Key Structure" :default "AnyKey"))
  (bind _plunger (`self.Plunger`))
  (:`Pressed`
    (`/Game/Blueprints/BP_Plunger.ChargePlunger` _plunger))
  (:`Released`
    (`/Game/Blueprints/BP_Plunger.StopCharge` _plunger)))

(fn `UserConstructionScript`)