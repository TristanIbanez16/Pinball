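; Plunger actor, apparently for pinball, that pulls back while charging and snaps back on release.
; ChargePlunger plays a timeline that lerps the Plunger component up to 150 units along local Y.
; StopCharge halts the timeline and uses MoveComponentTo to return the plunger over a tenth of a second.
; GetBallSpawnLocation converts BallLocation from actor space to world space for spawning balls.
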(event `ChargePlunger`
  (bind (_direction _chargealpha) (`Timeline|ChargeTimeline` :!via `PlayFromStart` :!label _label)
    (:`Update`
      (`SceneComponent.K2_SetRelativeLocation` (`self.Plunger`) (`KismetMathLibrary.VLerp` (0.0 0.0 0.0) (0.0 150.0 0.0) _chargealpha) false false))))

(event `StopCharge`
  (`|ExecutionSequence`
    (:`then_0`
      (goto _label :!via `Stop`))
    (:`then_1`
      (`KismetSystemLibrary.MoveComponentTo` (`self.Plunger`) (0.0 0.0 0.0) (struct) false false 0.1))))

(fn `GetBallSpawnLocation`
  (returns (BallSpawn :type "Vector Structure"))
  (return (`KismetMathLibrary.TransformLocation` (`self.GetTransform`) (`self.BallLocation`))))

(fn `UserConstructionScript`)